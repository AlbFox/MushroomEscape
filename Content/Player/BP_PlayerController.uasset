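; Player controller that sets up the player's camera and manages the game's UI widgets.
; On BeginPlay it spawns an Actor_Camera at a fixed height, possesses it, and adds the score and in-game HUD widgets to the viewport.
; EndGame flags the Map as game over and adds a W_HUD widget, while SetScore refreshes the stored score widget if it is valid.
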(event `self.ReceiveBeginPlay`
  (bind _returnvalue (`|SpawnActorFromClass` "/Game/Player/Actor_Camera.Actor_Camera_C" (`KismetMathLibrary.MakeTransform` (0.0 0.0 450.0)) "Undefined" "OverrideRootScale" null null))
  (`self.Possess` _returnvalue)
  (bind _returnvalue_2 (`|CreateWidget` "/Game/MushroomMap/Widgets/W_Score.W_Score_C"))
  (bind _output_get (set `self.Score` _returnvalue_2))
  (`UserWidget.AddToViewport` _output_get 0)
  (bind _returnvalue_3 (`|CreateWidget` "/Game/Player/W_InGameHUD.W_InGameHUD_C"))
  (`UserWidget.AddToViewport` _returnvalue_3 0))

(event `EndGame`
  (set `/Game/MushroomMap/Actor_Map.GameOver` true (`self.Map`))
  (bind _returnvalue (`|CreateWidget` "/Game/MushroomMap/Widgets/W_HUD.W_HUD_C"))
  (`UserWidget.AddToViewport` _returnvalue 0))

(event `SetScore`
  (bind _score (`self.Score`))
  (`/Engine/EditorBlueprintResources/StandardMacros.IsValid` _score
    (:`Is Valid`
      (`/Game/MushroomMap/Widgets/W_Score.Refresh` _score))))

(fn `UserConstructionScript`)